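; Player controller that rolls the BP_Player pawn's physics ball with keyboard input and steers the view with the mouse.
; Tick polls WASD and arrow keys, applying mass-independent forces to Ball1 along the camera's forward and right vectors.
; Space applies an upward velocity impulse when CanJump is true and clears the flag, which this file never sets back.
; Mouse axes feed yaw and pitch input, with pitch inverted.
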(event EventBeginPlay
  (bind _asbp_player (Utilities|Casting|CastToBP_Player (Pawn|GetControlledPawn)))
  (Variables|Default|SetBP%20Player _asbp_player))

(event EventTick
  (params (DeltaSeconds :type Float%20%28single-precision%29))
  (bind _bp_player (Variables|Default|GetBP%20Player))
  (bind _bp_player_2 (Variables|Default|GetBP%20Player))
  (bind _bp_player_3 (Variables|Default|GetBP%20Player))
  (bind _bp_player_4 (Variables|Default|GetBP%20Player))
  (bind _bp_player_5 (Variables|Default|GetBP%20Player))
  (bind _bp_player_6 (Variables|Default|GetBP%20Player))
  (bind _bp_player_7 (Variables|Default|GetBP%20Player))
  (bind _bp_player_8 (Variables|Default|GetBP%20Player))
  (Utilities|FlowControl|Sequence
    (:then_0
      ;[1 1 1] HANDLE W KEY
      (if (Game|Player|IsInputKeyDown "W")
        (Physics|AddForce (Variables|/Game/BP_Player.BP_Player_C|GetBall1 _bp_player_4) (* (Math|Vector|GetForwardVector (Variables|/Game/BP_Player.BP_Player_C|GetCamera _bp_player_4)) 1e+03) "None" true)))
    (:then_1
      ;[1 1 1] HANDLE S KEY
      (if (Game|Player|IsInputKeyDown "S")
        (Physics|AddForce (Variables|/Game/BP_Player.BP_Player_C|GetBall1 _bp_player_6) (* (Math|Vector|GetForwardVector (Variables|/Game/BP_Player.BP_Player_C|GetCamera _bp_player_6)) -1e+03) "None" true)))
    (:then_2
      ;[1 1 1] HANDLE A KEY
      (if (Game|Player|IsInputKeyDown "A")
        (Physics|AddForce (Variables|/Game/BP_Player.BP_Player_C|GetBall1 _bp_player_7) (* (Math|Vector|GetRightVector (Variables|/Game/BP_Player.BP_Player_C|GetCamera _bp_player_7)) -1e+03) "None" true)))
    (:then_3
      ;[1 1 1] HANDLE D KEY
      (if (Game|Player|IsInputKeyDown "D")
        (Physics|AddForce (Variables|/Game/BP_Player.BP_Player_C|GetBall1 _bp_player_8) (* (Math|Vector|GetRightVector (Variables|/Game/BP_Player.BP_Player_C|GetCamera _bp_player_8)) 1e+03) "None" true)))
    (:then_4
      ;[1 1 1] HANDLE UP KEY
      (if (Game|Player|IsInputKeyDown "Up")
        (Physics|AddForce (Variables|/Game/BP_Player.BP_Player_C|GetBall1 _bp_player_2) (* (Math|Vector|GetForwardVector (Variables|/Game/BP_Player.BP_Player_C|GetCamera _bp_player_2)) 1e+03) "None" true)))
    (:then_5
      ;[1 1 1] HANDLE DOWN KEY
      (if (Game|Player|IsInputKeyDown "Down")
        (Physics|AddForce (Variables|/Game/BP_Player.BP_Player_C|GetBall1 _bp_player_3) (* (Math|Vector|GetForwardVector (Variables|/Game/BP_Player.BP_Player_C|GetCamera _bp_player_3)) -1e+03) "None" true)))
    (:then_6
      ;[1 1 1] HANDLE LEFT KEY
      (if (Game|Player|IsInputKeyDown "Left")
        (Physics|AddForce (Variables|/Game/BP_Player.BP_Player_C|GetBall1 _bp_player_5) (* (Math|Vector|GetRightVector (Variables|/Game/BP_Player.BP_Player_C|GetCamera _bp_player_5)) -1e+03) "None" true)))
    (:then_7
      ;[1 1 1] HANDLE RIGHT KEY
      (if (Game|Player|IsInputKeyDown "Right")
        (Physics|AddForce (Variables|/Game/BP_Player.BP_Player_C|GetBall1 _bp_player) (* (Math|Vector|GetRightVector (Variables|/Game/BP_Player.BP_Player_C|GetCamera _bp_player)) 1e+03) "None" true)))))

(event Input|MouseEvents|MouseX
  (params (AxisValue :type Float%20%28single-precision%29))
  (Class|PlayerController|AddYawInput AxisValue))

(event Input|MouseEvents|MouseY
  (params (AxisValue :type Float%20%28single-precision%29))
  (Class|PlayerController|AddPitchInput (* AxisValue -1.0)))

(event Input|KeyboardEvents|SpaceBar
  (params (Key :type Key%20Structure))
  ;[1 1 1] JUMP SPACEBAR
  (:Pressed
    (if (Variables|Default|GetCanJump)
      (Variables|Default|SetCanJump false)
      (Physics|AddImpulse (Variables|/Game/BP_Player.BP_Player_C|GetBall1 (Variables|Default|GetBP%20Player)) "0, 0,1000.000000" "None" true))))

(fn ConstructionScript)