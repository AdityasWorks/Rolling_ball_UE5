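; Game mode that runs a timed collection level, winning when the score equals the number of BP_Cube actors and losing when the countdown runs out.
; BeginPlay creates the WBP_GameUI widget and starts a looping 0.01-second timer that decrements Time and updates its text.
; IncrementScore updates the score and checks for a win.
; Either outcome calls a DoOnce-guarded end screen that pauses the timer, reveals result buttons and switches to UI input.
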(event Custom|Increment%20Score
  (bind _output_get (Variables|Default|SetScore (+ (Variables|Default|GetScore) 1)))
  (Rendering|Components|TextRender|SetText (Variables|/Game/WBP_GameUI.WBP_GameUI_C|GetScoreText (Variables|Default|GetWidget%20Reference)) (Utilities|Text|ToText(Integer) _output_get))
  (if (== _output_get (Variables|Default|GetMAX%20SCORE))
    (CallFunction|ShowEndScreen "YOU WIN")))

(event Custom|Timer%20Event
  (bind _output_get (Variables|Default|SetTime (- (Variables|Default|GetTime) 1)))
  (Rendering|Components|TextRender|SetText (Variables|/Game/WBP_GameUI.WBP_GameUI_C|GetTimeText (Variables|Default|GetWidget%20Reference)) (Utilities|Text|ToText(Integer) _output_get))
  (if (<= _output_get 0)
    (CallFunction|ShowEndScreen "GAME OVER")))

(event Custom|Show%20End%20Screen
  (params (Result%20Text :type Text))
  (bind _returnvalue (Game|GetPlayerController 0))
  (bind _widget_reference (Variables|Default|GetWidget%20Reference))
  (Utilities|FlowControl|DoOnce false
    (:Completed
      (Utilities|Time|PauseTimerbyHandle (Variables|Default|GetTimer))
      (Rendering|Components|TextRender|SetText (Variables|/Game/WBP_GameUI.WBP_GameUI_C|GetResultText _widget_reference) Result%20Text)
      (Widget|SetVisibility (Variables|/Game/WBP_GameUI.WBP_GameUI_C|GetBgBlur _widget_reference) "SelfHitTestInvisible")
      (Widget|SetVisibility (Variables|/Game/WBP_GameUI.WBP_GameUI_C|GetReplayButton _widget_reference) "Visible")
      (Widget|SetVisibility (Variables|/Game/WBP_GameUI.WBP_GameUI_C|GetNEXTButton _widget_reference) "Visible")
      (Input|SetInputModeUIOnly _returnvalue (Variables|Default|GetWidget%20Reference) "DoNotLock" true)
      (Variables|/Script/Engine.PlayerController|SetbShowMouseCursor _returnvalue true))))

(event EventBeginPlay
  (Input|SetInputModeGameOnly (Game|GetPlayerController 0) true)
  (bind _outactors (Actor|GetAllActorsOfClass "/Game/BP_Cube.BP_Cube_C"))
  (Variables|Default|SetMAX%20SCORE (Utilities|Array|Length _outactors))
  (bind _returnvalue (UserInterface|CreateWidget "/Game/WBP_GameUI.WBP_GameUI_C"))
  (bind _output_get (Variables|Default|SetWidget%20Reference _returnvalue))
  (UserInterface|Viewport|AddtoViewport _output_get 0)
  (bind _returnvalue_2 (Utilities|Time|SetTimerbyEvent (delegate Custom|Timer%20Event) 0.01 true))
  (Variables|Default|SetTimer _returnvalue_2))

(fn ConstructionScript)